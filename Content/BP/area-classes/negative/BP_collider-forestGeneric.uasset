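; Negative area collider for a generic forest that makes AI characters fearful when they enter it.
; On begin overlap it casts the other actor to AIpawn_characterDefault, sets its DominantEmotion to "fear", and prints the collider's class name as orange debug text.
; A LocationDecision call on the pawn is present but never runs, and the construction script only calls the parent.
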(event Collision|EventActorBeginOverlap
  (params (OtherActor :type Actor%20Object%20Reference))
  (bind _asaipawn_character_default (Utilities|Casting|CastToAIpawn_characterDefault OtherActor))
  (Variables|/Script/NeuroSim.AIpawn_characterDefault|SetdominantEmotion _asaipawn_character_default "fear")
  (Development|PrintText (Utilities|Text|ToText(String) (Utilities|GetClassDisplayName (Utilities|GetClass self))) true true "(R=1.000000,G=0.332501,B=0.018288,A=1.000000)"))

(fn ConstructionScript
  (|CallParentFunction))